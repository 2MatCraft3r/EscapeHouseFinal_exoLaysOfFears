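; BP_Door01 is a door Blueprint that swings its static mesh between 90 and 0 degrees of yaw.
; The custom openDoor event toggles IsClosed, playing or reversing a Timeline that drives the yaw Lerp.
; Timeline updates feed a one-second retriggerable delay, which clears IsClosed and reverses the Timeline, returning the door automatically once movement settles.
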(event Custom|openDoor
  (if (Variables|Default|GetIsClosed)
    (Variables|Default|SetIsClosed false)
    (bind _newtrack_0 (Timeline|Timeline Reverse)
      (:Update
        (Transformation|SetRelativeRotation (Variables|Default|GetSM_GTJ_Door08C_StaticMeshComponent0) (Math|Rotator|MakeRotator 0.0 0.0 (Math|Float|Lerp 9e+01 0.0 _newtrack_0)) false false)
        (Utilities|FlowControl|RetriggerableDelay 1.0)
        (Variables|Default|SetIsClosed false)
        (Timeline|Timeline Reverse)))
    (else
      (Variables|Default|SetIsClosed true)
      (Timeline|Timeline Play))))

(event EventBeginPlay)

(event Collision|EventActorBeginOverlap
  (params (OtherActor :type Actor%20Object%20Reference)))

(event EventTick
  (params (DeltaSeconds :type Float%20%28single-precision%29)))

(fn ConstructionScript)