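; A key-locked door actor that toggles open and closed when its openDoor event is called.
; If the referenced Key reports HaveKey, a Timeline plays or reverses to drive the mesh's relative yaw, scaled by RotationAngle plus a fixed offset.
; Without the key it prints a French message saying one is needed.
; The starting yaw is saved on BeginPlay but never applied to the rotation.
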(event Custom|openDoor
  (if (Variables|/Game/BP_Key.BP_Key_C|GetHaveKey (Variables|Default|GetKey))
    (if (Variables|Default|GetIsClosed)
      (Variables|Default|SetIsClosed false)
      (bind _newtrack_0 (Timeline|Timeline Play)
        (:Update
          (Transformation|SetRelativeRotation (Variables|Default|GetSM_GTJ_Door08C_StaticMeshComponent0) (Math|Rotator|MakeRotator 0.0 0.0 (* _newtrack_0 (+ (Variables|Default|GetRotationAngle) 9e+01) 1.0)) false false)))
      (else
        (Variables|Default|SetIsClosed true)
        (Timeline|Timeline Reverse)))
    (else
      (Development|PrintString "Il faut une clé"))))

(event EventBeginPlay
  (Variables|Default|SetInitialRotate (.yaw (Variables|/Script/Engine.SceneComponent|GetRelativeRotation (Variables|Default|GetSM_GTJ_Door08C_StaticMeshComponent0)))))

(event Collision|EventActorBeginOverlap
  (params (OtherActor :type Actor%20Object%20Reference)))

(event EventTick
  (params (DeltaSeconds :type Float%20%28single-precision%29)))

(fn ConstructionScript)